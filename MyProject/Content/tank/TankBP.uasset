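; Player-controllable tank Blueprint that wires its components together and maps input to driving, camera control and firing.
; On BeginPlay it passes barrel and turret to the TankAim1 aiming component and both tracks to TankMovement.
; Turret axes orbit and pitch the camera rig via RotationParent and SpringArm, with frame-time-scaled zoom on arm length.
; Drive axes forward movement intent to TankMovement, and fire calls TankAim1.
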(event Collision|EventActorBeginOverlap
  (params (OtherActor :type Actor%20Object%20Reference)))

(event EventTick
  (params (DeltaSeconds :type Float%20%28single-precision%29)))

(event EventBeginPlay
  (Class|TankAimComponent|InitialiseAim (Variables|Default|GetTankAim1) (Variables|Default|GetTankBarrel) (Variables|Default|GetTankTurret))
  (Class|TankMovementComponent|Initialise (Variables|Default|GetTankMovement) (Variables|Default|GetLTrack) (Variables|Default|GetRTrack)))

(event Input|ActionEvents|InputActionfire
  (params (Key :type Key%20Structure :default "AnyKey"))
  ;[1 1 1] Input Binding
  (:Pressed
    (Class|TankAimComponent|Fire (Variables|Default|GetTankAim1))))

(event Input|AxisEvents|InputAxisTurretRotation
  (params (AxisValue :type Float%20%28single-precision%29))
  ;[1 1 1] Input Binding
  (Transformation|AddLocalRotation (Variables|Default|GetRotationParent) (Math|Rotator|MakeRotator 0.0 0.0 (* AxisValue (Utilities|Time|GetWorldDeltaSeconds) 1e+02)) false false))

(event Input|AxisEvents|InputAxisForwardBackward
  (params (AxisValue :type Float%20%28single-precision%29))
  ;[1 1 1] Input Binding
  (Class|TankMovementComponent|IntendMoveForward (Variables|Default|GetTankMovement) AxisValue))

(event Input|AxisEvents|InputAxiszoomIn
  (params (AxisValue :type Float%20%28single-precision%29))
  (bind _springarm (Variables|Default|GetSpringArm))
  ;[1 1 1] Input Binding
  (Variables|/Script/Engine.SpringArmComponent|SetTargetArmLength _springarm (+ (* (Utilities|Time|GetWorldDeltaSeconds) AxisValue 5e+01) (Variables|/Script/Engine.SpringArmComponent|GetTargetArmLength _springarm))))

(event Input|AxisEvents|InputAxisRotate
  (params (AxisValue :type Float%20%28single-precision%29))
  ;[1 1 1] Input Binding
  (Class|TankMovementComponent|IntendRotateRight (Variables|Default|GetTankMovement) AxisValue))

(event Input|AxisEvents|InputAxisTurretElevation
  (params (AxisValue :type Float%20%28single-precision%29))
  ;[1 1 1] Input Binding
  (Transformation|AddLocalRotation (Variables|Default|GetSpringArm) (Math|Rotator|MakeRotator 0.0 (* AxisValue (Utilities|Time|GetWorldDeltaSeconds) 5e+01) 0.0) false false))

(fn ConstructionScript
  (Development|PrintString "Donkey Constractur BP" false true "(R=1.000000,G=0.000000,B=0.864500,A=1.000000)"))